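; LevelBox_BP is a Blueprint box that detects when the mouse cursor hovers over it.
; On BeginPlay it enables mouse-over events on the first player controller and prints a debug string.
; Cursor enter and exit events on the COLLISION component set IsCursorHovering, which this Blueprint never reads.
; Those events and MainBox's cursor-enter event also print a "Hello" debug message.
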(event `self.ReceiveBeginPlay`
  (`KismetSystemLibrary.PrintString` "Hello")
  (set `PlayerController.bEnableMouseOverEvents` true (`GameplayStatics.GetPlayerController` 0)))

(event `self.MainBox.OnBeginCursorOver`
  (params (TouchedComponent :type "PrimitiveComponent Object Reference"))
  (`KismetSystemLibrary.PrintString` "Hello"))

(event `self.COLLISION.OnBeginCursorOver`
  (params (TouchedComponent :type "PrimitiveComponent Object Reference"))
  (set `self.isCursorHovering` true)
  (`KismetSystemLibrary.PrintString` "Hello"))

(event `self.COLLISION.OnEndCursorOver`
  (params (TouchedComponent :type "PrimitiveComponent Object Reference"))
  (set `self.isCursorHovering` false)
  (`KismetSystemLibrary.PrintString` "Hello"))

(fn `UserConstructionScript`)