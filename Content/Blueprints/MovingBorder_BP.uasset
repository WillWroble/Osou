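; MovingBorder_BP is a border actor with a Fire particle effect whose spawn rate follows the actor's scale.
; BeginPlay sets the effect's RelativeSpawnRate to one, then every Tick overwrites it with the actor's X scale.
; Unconnected nodes for RelativeParticleScale never run, and the file contains no movement logic.
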(event `self.ReceiveBeginPlay`
  (`NiagaraComponent.SetVariableFloat` (`self.Fire`) "RelativeSpawnRate" 1.0))

(event `self.ReceiveTick`
  (params (DeltaSeconds :type "Float (single-precision)"))
  (`NiagaraComponent.SetVariableFloat` (`self.Fire`) "RelativeSpawnRate" (.x (`self.GetActorScale3D`))))

(fn `UserConstructionScript`)