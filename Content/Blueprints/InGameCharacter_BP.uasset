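; In-game character actor that displays a level-specific Paper2D flipbook character, such as Sakuya, Flandere, Rin or Cirno.
; InitAnims picks idle and attack flipbooks by LevelIndexBP, adjusting scale for some characters, or hides the actor and disables collision.
; PlayAnim events set non-looping attack flipbooks, and OnFinishedPlaying restores the looping default.
; Other events switch that default between Idle, Float and Dash, reapplying rotation for the latter two.
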(event `self.ReceiveBeginPlay`)

(event `self.InitAnims`
  (bind _idle (`self.idle`))
  (switch `int` (`self.levelIndex_BP`)
    (:`Default`
      (set `self.idle` "/Game/Animations/Sakuya/idle/sakuya_idle.sakuya_idle" :!label _label)
      (set `self.knife1` "/Game/Animations/Sakuya/KnifeThrow1/sakuya_knife1.sakuya_knife1")
      (set `self.knife2` "/Game/Animations/Sakuya/KnifeThrow2/SakuyaKnife2.SakuyaKnife2")
      (`PaperFlipbookComponent.SetFlipbook` (`self.Anim`) (`self.idle`) :!label _label_2)
      (`PaperFlipbookComponent.PlayFromStart` (`self.Anim`))
      (set `self.defaultAnim` _idle)
      (set `self.float` _idle))
    (:`0`
      (`SceneComponent.SetVisibility` (`self.DefaultSceneRoot`) false true :!label _label_3)
      (`PrimitiveComponent.SetCollisionEnabled` (`self.Anim`) "NoCollision"))
    (:`1`
      (set `self.idle` "/Game/Animations/Fladere/Idle/FlandereIdleFB.FlandereIdleFB")
      (set `self.knife1` "/Game/Animations/Fladere/Attack1/FlandereAttack1_FB.FlandereAttack1_FB")
      (set `self.knife2` "/Game/Animations/Fladere/Attack2/FladereAttack2FB.FladereAttack2FB")
      (set `self.knife3` "/Game/Animations/Fladere/Attack3/FlandereAttack3FB.FlandereAttack3FB")
      (set `self.knife4` "/Game/Animations/Fladere/Laugh/LaughFB.LaughFB")
      (`SceneComponent.SetRelativeScale3D` (`self.Anim`) (-1.0 1.0 1.0))
      (goto _label_2))
    (:`2`
      (goto _label_3))
    (:`3`
      (goto _label_3))
    (:`4`
      (goto _label_3))
    (:`5`
      (goto _label))
    (:`6`
      (set `self.idle` "/Game/Animations/Rin/Idle/rin_idleFB.rin_idleFB")
      (set `self.knife1` "/Game/Animations/Rin/Attack1/RinAttack1FB.RinAttack1FB")
      (set `self.knife2` "/Game/Animations/Rin/Attack1/RinAttack1FB.RinAttack1FB")
      (`self.SetActorScale3D` (2.5 2.5 2.5))
      (goto _label_2))
    (:`7`
      (set `self.idle` "/Game/Animations/Cirno/Idle/Cirno_idle_FB.Cirno_idle_FB")
      (set `self.knife1` "/Game/Animations/Cirno/Attack/cirno_attack1_FB.cirno_attack1_FB")
      (set `self.knife2` "/Game/Animations/Sakuya/KnifeThrow2/SakuyaKnife2.SakuyaKnife2")
      (`self.SetActorScale3D` (2.0 2.0 2.0))
      (goto _label_2))
    (:`8`
      (goto _label_3))))

(event `self.SetDefaultAnimToFloat`
  (set `self.initialRotation` (`SceneComponent.RelativeRotation` (`self.Anim`)))
  (set `self.defaultAnim` (`self.float`))
  (`PaperFlipbookComponent.SetFlipbook` (`self.Anim`) (`self.defaultAnim`) :!label _label_4)
  (`PaperFlipbookComponent.SetLooping` (`self.Anim`) true)
  (`PaperFlipbookComponent.PlayFromStart` (`self.Anim`))
  (if (or (== (`self.defaultAnim`) (`self.dash`)) (== (`self.defaultAnim`) (`self.float`)))
    (`SceneComponent.K2_SetRelativeRotation` (`self.Anim`) (`self.initialRotation`) false false)
    (`KismetSystemLibrary.PrintString` "BACK TO DASH")
    (else
      (set `self.dontResetRotation` false))))

(event `self.SetDefaultAnimToDash`
  (set `self.initialRotation` (`SceneComponent.RelativeRotation` (`self.Anim`)))
  (set `self.defaultAnim` (`self.dash`))
  (goto _label_4))

(event `self.SetDefaultAnimToIdle`
  (set `self.defaultAnim` (`self.idle`))
  (goto _label_4))

(event `self.Anim.OnFinishedPlaying`
  (goto _label_4))

(event `self.PlayAnimOne`
  (bind _anim (`self.Anim`))
  (set `self.dontResetRotation` true)
  (`PaperFlipbookComponent.SetLooping` (`self.Anim`) false :!label _label_5)
  (`PaperFlipbookComponent.SetFlipbook` _anim (`self.knife1`))
  (`PaperFlipbookComponent.PlayFromStart` _anim))

(event `self.StartDashAnim`
  (`PaperFlipbookComponent.SetFlipbook` (`self.Anim`) (`self.dash`))
  (`PaperFlipbookComponent.SetLooping` (`self.Anim`) true)
  (`PaperFlipbookComponent.PlayFromStart` (`self.Anim`)))

(event `self.EndDashAnim`
  (`PaperFlipbookComponent.SetLooping` (`self.Anim`) false))

(event `self.PlayAnimFive`
  (set `self.dontResetRotation` true)
  (goto _label_5))

(event `self.PlayAnimTwo`
  (set `self.dontResetRotation` true)
  (`PaperFlipbookComponent.SetLooping` (`self.Anim`) false)
  (`PaperFlipbookComponent.SetFlipbook` (`self.Anim`) (`self.knife2`)))

(event `self.PlayAnimThree`
  (set `self.dontResetRotation` true)
  (`PaperFlipbookComponent.SetLooping` (`self.Anim`) false)
  (`PaperFlipbookComponent.SetFlipbook` (`self.Anim`) (`self.knife3`)))

(event `self.PlayAnimFour`
  (set `self.dontResetRotation` true)
  (`PaperFlipbookComponent.SetLooping` (`self.Anim`) false)
  (`PaperFlipbookComponent.SetFlipbook` (`self.Anim`) (`self.knife4`)))

(fn `UserConstructionScript`)