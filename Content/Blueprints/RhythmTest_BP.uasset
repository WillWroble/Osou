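; RhythmTest_BP is a Blueprint that shows captioned text on screen through a RhythmTestUI widget.
; On BeginPlay it creates the widget, stores it and adds it to the viewport.
; FadeinText sets the widget's Caption from a Content value and plays the FadeTextIn animation, while FadeOutText plays FadeTextOut.
; Overlap and Tick events are unused.
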(event `self.ReceiveBeginPlay`
  (bind _returnvalue (`|CreateWidget` "/Game/Widget/RhythmTestUI.RhythmTestUI_C"))
  (set `self.Widget` _returnvalue)
  (`UserWidget.AddToViewport` (`self.Widget`) 0))

(event `self.FadeInText`
  (bind _widget (`self.Widget`))
  (`TextBlock.SetText` (`/Game/Widget/RhythmTestUI.caption` (`self.Widget`)) (`KismetTextLibrary.Conv_StringToText` (`self.content`)))
  (`UserWidget.PlayAnimation` _widget (`/Game/Widget/RhythmTestUI.FadeTextIn` _widget) 0.0 1 "Forward" 1.0 false))

(event `self.FadeOutText`
  (bind _widget (`self.Widget`))
  (`UserWidget.PlayAnimation` _widget (`/Game/Widget/RhythmTestUI.FadeTextOut` _widget) 0.0 1 "Forward" 1.0 false))

(fn `UserConstructionScript`)