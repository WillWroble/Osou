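; Rhythm-game actor that creates and drives the in-game HUD: metronome swings, timing popups, health icons, captions and pause menu.
; On level finish it combines HScore and RScore into a weighted score, shows an S-to-D grade and positions a pointer on the score widget.
; It asynchronously loads the save slot, creating a save object if loading fails, and writes score and grade only when the level's best is beaten.
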(event `self.CloseWidget`
  (bind _ingamehudref (`self.inGameHUDRef`))
  (bind _ingamehudref_2 (`self.inGameHUDRef`))
  (`Widget.SetVisibility` (`/Game/Widget/InGameHUD.W_LevelScore` (`self.inGameHUDRef`)) "Collapsed")
  (`|ExecutionSequence`
    (:`then_0`
      (`Widget.SetVisibility` (`/Game/Widget/InGameHUD.H_1` _ingamehudref) "Visible"))
    (:`then_1`
      (`Widget.SetVisibility` (`/Game/Widget/InGameHUD.H_2` _ingamehudref) "Visible"))
    (:`then_2`
      (`Widget.SetVisibility` (`/Game/Widget/InGameHUD.H_3` _ingamehudref) "Visible"))
    (:`then_3`
      (`Widget.SetVisibility` (`/Game/Widget/InGameHUD.H_4` _ingamehudref) "Visible"))
    (:`then_4`
      (`Widget.SetVisibility` (`/Game/Widget/InGameHUD.H_5` _ingamehudref_2) "Visible"))
    (:`then_5`
      (`Widget.SetVisibility` (`/Game/Widget/InGameHUD.H_6` _ingamehudref_2) "Visible"))
    (:`then_6`
      (`Widget.SetVisibility` (`/Game/Widget/InGameHUD.H_7` _ingamehudref_2) "Visible"))
    (:`then_7`
      (`Widget.SetVisibility` (`/Game/Widget/InGameHUD.H_8` _ingamehudref_2) "Visible"))))

(event `self.OnFinishLevel`
  (bind _currentlevel (`self.currentLevel`))
  (bind _currentsave (`self.currentSave`))
  (bind _score (`self.score`))
  (bind _w_levelscore (`/Game/Widget/InGameHUD.W_LevelScore` (`self.inGameHUDRef`)))
  (bind _scores (`MySaveGame.scores` (`self.currentSave`)))
  (bind _grades (`MySaveGame.grades` (`self.currentSave`)))
  (bind _textblock_63 (`/Game/Widget/W_LevelScore.TextBlock_63` (`/Game/Widget/InGameHUD.W_LevelScore` (`self.inGameHUDRef`))))
  (bind _returnvalue (* (- 100 (* (`self.hScore`) 10)) (`KismetMathLibrary.MultiplyMultiply_FloatFloat` (/ (`self.rScore`) 100.0) 0.25)))
  (bind _returnvalue_2 (> (`self.score`) (`|GetArrayItem` _scores _currentlevel)))
  (`Widget.SetVisibility` _w_levelscore "Visible")
  (`TextBlock.SetText` (`/Game/Widget/W_LevelScore.TextBlock_3886` _w_levelscore) (`KismetTextLibrary.Conv_IntToText` (`self.hScore`)))
  (`TextBlock.SetText` (`/Game/Widget/W_LevelScore.TextBlock_4687` _w_levelscore) (`KismetTextLibrary.Conv_StringToText` (`KismetStringLibrary.Concat_StrStr` (`KismetStringLibrary.Conv_DoubleToString` (`self.rScore`)) "%")))
  (set `self.score` _returnvalue)
  (`TextBlock.SetText` (`/Game/Widget/W_LevelScore.TextBlock_5113` _w_levelscore) (`KismetTextLibrary.Conv_DoubleToText` _returnvalue "HalfToEven"))
  (`KismetSystemLibrary.PrintString` "FINISHED LEVEL" true false)
  (`Widget.SetRenderTranslation` (`/Game/Widget/W_LevelScore.Pointer` (`/Game/Widget/InGameHUD.W_LevelScore` (`self.inGameHUDRef`))) (`KismetMathLibrary.MakeVector2D` (+ -310.0 (`KismetMathLibrary.Conv_IntToDouble` (* (`self.hScore`) 88))) (+ -55.0 (* (/ (- (`self.rScore`) 66.0) 34.0) 262.0))))
  (bind (_savegame _bsuccess) (`AsyncActionHandleSaveGame.AsyncLoadGameFromSlot` "osou_save")
    (:`Completed`
      (if _bsuccess
        (bind _asmy_save_game (cast `MySaveGame` _savegame))
        (set `self.currentSave` _asmy_save_game)
        (else
          (bind _returnvalue_3 (`GameplayStatics.CreateSaveGameObject` "/Game/Blueprints/MySaveGame_BP.MySaveGame_BP_C"))
          (`KismetArrayLibrary.Array_Resize` (`MySaveGame.grades` _returnvalue_3) 72)
          (`KismetArrayLibrary.Array_Resize` (`MySaveGame.scores` _returnvalue_3) 72)
          (set `self.currentSave` _returnvalue_3)))
      (if (>= (`self.score`) 93.669998)
        (`TextBlock.SetText` _textblock_63 "S")
        (`TextBlock.SetColorAndOpacity` _textblock_63 (make `SlateColor` (struct :`R` 0.23074 :`G` 0.039546 :`B` 0.715693 :`A` 1.0)))
        (if _returnvalue_2
          (`KismetArrayLibrary.Array_Set` _scores _currentlevel _score true)
          (`KismetArrayLibrary.Array_Set` _grades _currentlevel 1 true)
          (bind (_savegame_2 _bsuccess_2) (`AsyncActionHandleSaveGame.AsyncSaveGameToSlot` _currentsave "osou_save")
            (:`Completed`
              (if _bsuccess_2
                (`KismetSystemLibrary.PrintString` "SAVE SUCESSFUL" true false :!label _label)
                (else
                  (`KismetSystemLibrary.PrintString` "SAVE FAILED" true false :!label _label_2))))))
        (elif (>= (`self.score`) 84.306999)
          (`TextBlock.SetText` _textblock_63 "A")
          (`TextBlock.SetColorAndOpacity` _textblock_63 (make `SlateColor` (struct :`R` 0.022174 :`G` 0.366253 :`B` 0.022174 :`A` 1.0)))
          (if _returnvalue_2
            (`KismetArrayLibrary.Array_Set` _scores _currentlevel _score true)
            (`KismetArrayLibrary.Array_Set` _grades _currentlevel 2 true)
            (bind (_savegame_3 _bsuccess_3) (`AsyncActionHandleSaveGame.AsyncSaveGameToSlot` _currentsave "osou_save")
              (:`Completed`
                (if _bsuccess_3
                  (goto _label)
                  (else
                    (goto _label_2))))))
          (elif (>= (`self.score`) 67.797997)
            (`TextBlock.SetText` _textblock_63 "B")
            (`TextBlock.SetColorAndOpacity` _textblock_63 (make `SlateColor` (struct :`R` 0.238398 :`G` 0.366253 :`B` 0.022174 :`A` 1.0)))
            (if _returnvalue_2
              (`KismetArrayLibrary.Array_Set` _scores _currentlevel _score true)
              (`KismetArrayLibrary.Array_Set` _grades _currentlevel 3 true)
              (bind (_savegame_4 _bsuccess_4) (`AsyncActionHandleSaveGame.AsyncSaveGameToSlot` _currentsave "osou_save")
                (:`Completed`
                  (if _bsuccess_4
                    (goto _label)
                    (else
                      (goto _label_2))))))
            (elif (>= (`self.score`) 46.837399)
              (`TextBlock.SetText` _textblock_63 "C")
              (`TextBlock.SetColorAndOpacity` _textblock_63 (make `SlateColor` (struct :`R` 0.814847 :`G` 0.708376 :`B` 0.002428 :`A` 1.0)))
              (if _returnvalue_2
                (`KismetArrayLibrary.Array_Set` _scores _currentlevel _score true)
                (`KismetArrayLibrary.Array_Set` _grades _currentlevel 4 true)
                (bind (_savegame_5 _bsuccess_5) (`AsyncActionHandleSaveGame.AsyncSaveGameToSlot` _currentsave "osou_save")
                  (:`Completed`
                    (if _bsuccess_5
                      (goto _label)
                      (else
                        (goto _label_2))))))
              (else
                (`TextBlock.SetText` _textblock_63 "D")
                (`TextBlock.SetColorAndOpacity` _textblock_63 (make `SlateColor` (struct :`R` 0.814847 :`G` 0.002732 :`B` 0.002428 :`A` 1.0)))
                (if _returnvalue_2
                  (`KismetArrayLibrary.Array_Set` _scores _currentlevel _score true)
                  (`KismetArrayLibrary.Array_Set` _grades _currentlevel 5 true)
                  (bind (_savegame_6 _bsuccess_6) (`AsyncActionHandleSaveGame.AsyncSaveGameToSlot` _currentsave "osou_save")
                    (:`Completed`
                      (if _bsuccess_6
                        (goto _label)
                        (else
                          (goto _label_2))))))))))))))

(event `self.ReceiveBeginPlay`
  (bind _ingamehudref (`self.inGameHUDRef`))
  (bind _returnvalue (`|CreateWidget` "/Game/Widget/InGameHUD.InGameHUD_C"))
  (set `self.inGameHUDRef` _returnvalue)
  (set `self.Health` 1.0)
  (set `/Game/Widget/InGameHUD.actorRef` self (`self.inGameHUDRef`))
  (`UserWidget.AddToViewport` _ingamehudref 0)
  (set `self.widget` _ingamehudref)
  (`Widget.SetVisibility` (`/Game/Widget/InGameHUD.W_LevelScore` (`self.inGameHUDRef`)) "Collapsed"))

(event `self.OnBeatChange`
  (bind _ingamehudref (`self.inGameHUDRef`))
  (bind _metronomespeed (`self.metronomeSpeed`))
  (if (`self.isSwingRight`)
    (`UserWidget.PlayAnimation` _ingamehudref (`/Game/Widget/InGameHUD.SwingRight` _ingamehudref) 0.0 1 "Forward" _metronomespeed false)
    (set `self.isSwingRight` false)
    (else
      (`UserWidget.PlayAnimation` _ingamehudref (`/Game/Widget/InGameHUD.SwingLeft` _ingamehudref) 0.0 1 "Forward" _metronomespeed false)
      (set `self.isSwingRight` true))))

(event `self.OnSlightlyEarly`
  (bind _ingamehudref (`self.inGameHUDRef`))
  (bind _ingamehudref_2 (`self.inGameHUDRef`))
  (bind _textblock_0 (`/Game/Widget/InGameHUD.TextBlock_0` (`self.inGameHUDRef`)))
  (`UserWidget.StopAnimation` _ingamehudref (`/Game/Widget/InGameHUD.BigEarly` _ingamehudref))
  (`UserWidget.StopAnimation` _ingamehudref (`/Game/Widget/InGameHUD.BigLate` _ingamehudref))
  (`UserWidget.StopAnimation` _ingamehudref (`/Game/Widget/InGameHUD.LittleEarly` _ingamehudref))
  (`UserWidget.StopAnimation` _ingamehudref (`/Game/Widget/InGameHUD.LittleLate` _ingamehudref))
  (`UserWidget.StopAnimation` _ingamehudref (`/Game/Widget/InGameHUD.Perfect` _ingamehudref))
  (switch `int` (`self.PopupType`)
    (:`Default`
      (`TextBlock.SetText` _textblock_0 "PERFECT" :!label _label_3)
      (`UserWidget.PlayAnimation` _ingamehudref_2 (`/Game/Widget/InGameHUD.Perfect` _ingamehudref_2) 0.0 1 "Forward" 1.0 false))
    (:`0`
      (`TextBlock.SetText` _textblock_0 "EARLY")
      (`UserWidget.PlayAnimation` _ingamehudref_2 (`/Game/Widget/InGameHUD.BigEarly` _ingamehudref_2) 0.0 1 "Forward" 1.0 false))
    (:`1`
      (`TextBlock.SetText` _textblock_0 "EARLY")
      (`UserWidget.PlayAnimation` _ingamehudref_2 (`/Game/Widget/InGameHUD.LittleEarly` _ingamehudref_2) 0.0 1 "Forward" 1.0 false))
    (:`2`
      (`TextBlock.SetText` _textblock_0 "LATE")
      (`UserWidget.PlayAnimation` _ingamehudref_2 (`/Game/Widget/InGameHUD.BigLate` _ingamehudref_2) 0.0 1 "Forward" 1.0 false))
    (:`3`
      (`TextBlock.SetText` _textblock_0 "LATE")
      (`UserWidget.PlayAnimation` _ingamehudref_2 (`/Game/Widget/InGameHUD.LittleLate` _ingamehudref_2) 0.0 1 "Forward" 1.0 false))
    (:`4`
      (goto _label_3))))

(event `InputAction|Pause`
  (params (Key :type "Key Structure"))
  (:`Pressed`
    (`Widget.SetVisibility` (`/Game/Widget/InGameHUD.W_Pause` (`self.inGameHUDRef`)) "Visible")
    (`self.StopEverything`)))

(event `self.UpdateHealthBar`
  (bind _ingamehudref (`self.inGameHUDRef`))
  (bind _ingamehudref_2 (`self.inGameHUDRef`))
  (switch `int` (`self.hScore`)
    (:`0`
      (`Widget.SetVisibility` (`/Game/Widget/InGameHUD.H_1` _ingamehudref) "Collapsed"))
    (:`1`
      (`Widget.SetVisibility` (`/Game/Widget/InGameHUD.H_2` _ingamehudref) "Collapsed"))
    (:`2`
      (`Widget.SetVisibility` (`/Game/Widget/InGameHUD.H_3` _ingamehudref) "Collapsed"))
    (:`3`
      (`Widget.SetVisibility` (`/Game/Widget/InGameHUD.H_4` _ingamehudref) "Collapsed"))
    (:`4`
      (`Widget.SetVisibility` (`/Game/Widget/InGameHUD.H_5` _ingamehudref_2) "Collapsed"))
    (:`5`
      (`Widget.SetVisibility` (`/Game/Widget/InGameHUD.H_6` _ingamehudref_2) "Collapsed"))
    (:`6`
      (`Widget.SetVisibility` (`/Game/Widget/InGameHUD.H_7` _ingamehudref_2) "Collapsed"))
    (:`7`
      (`Widget.SetVisibility` (`/Game/Widget/InGameHUD.H_8` _ingamehudref_2) "Collapsed"))))

(event `self.FadeInText`
  (bind _ingamehudref (`self.inGameHUDRef`))
  (`TextBlock.SetText` (`/Game/Widget/InGameHUD.caption` (`self.inGameHUDRef`)) (`KismetTextLibrary.Conv_StringToText` (`self.content`)))
  (`UserWidget.PlayAnimation` _ingamehudref (`/Game/Widget/InGameHUD.FadeTextIn` _ingamehudref) 0.0 1 "Forward" 1.0 false))

(event `self.FadeOutText`
  (bind _ingamehudref (`self.inGameHUDRef`))
  (`UserWidget.PlayAnimation` _ingamehudref (`/Game/Widget/InGameHUD.FadeTextOut` _ingamehudref) 0.0 1 "Forward" 1.0 false))

(fn `UserConstructionScript`)