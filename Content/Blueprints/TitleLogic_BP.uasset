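; Title screen logic actor that starts the game's front end on BeginPlay and picks one of four music tracks at random.
; It async-loads the settings save, creating defaults if absent, then checks the game save and plays a faded intro info screen when none loads.
; It then sets the background material texture, shows the title widget linked to itself, enables VSync and applies the saved master volume.
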(event `self.ReceiveBeginPlay`
  (bind _a1 (`self.a1`))
  (bind _a1_2 (`self.a1`))
  (bind _infroscreenref (`self.infroScreenRef`))
  (`|ExecutionSequence`
    (:`then_0`
      (`ActorComponent.Activate` _a1 false)
      (bind (_savegame _bsuccess) (`AsyncActionHandleSaveGame.AsyncLoadGameFromSlot` "osou_settings")
        (:`Completed`
          (if _bsuccess
            (`KismetSystemLibrary.PrintString` "Save Found")
            (bind _assaved_settings_bp (cast `/Game/Blueprints/SavedSettings_BP` _savegame))
            (`KismetSystemLibrary.PrintString` (`KismetStringLibrary.Conv_DoubleToString` (`/Game/Blueprints/SavedSettings_BP.Master Volume` _assaved_settings_bp)))
            (else
              (`KismetSystemLibrary.PrintString` "Create New Settings Save")
              (bind _returnvalue (`GameplayStatics.CreateSaveGameObject` "/Game/Blueprints/SavedSettings_BP.SavedSettings_BP_C"))
              (set `/Game/Blueprints/SavedSettings_BP.Master Volume` 0.5 _returnvalue)
              (set `/Game/Blueprints/SavedSettings_BP.Backround Brightness` 1.0 _returnvalue)
              (`AsyncActionHandleSaveGame.AsyncSaveGameToSlot` _returnvalue "osou_settings"
                (:`Completed`
                  _))))
          (bind (_savegame_2 _bsuccess_2) (`AsyncActionHandleSaveGame.AsyncLoadGameFromSlot` "osou_save")
            (:`Completed`
              (if (not _bsuccess_2)
                (`PlayerCameraManager.StartCameraFade` :`self` (`PlayerController.PlayerCameraManager` (`GameplayStatics.GetPlayerController` 0)) :`ToAlpha` 1.0 :`Duration` 0.01 :`bHoldWhenFinished` true)
                (bind _returnvalue_2 (`|CreateWidget` "/Game/Widget/InfoScreen.InfoScreen_C"))
                (bind _output_get (set `self.infroScreenRef` _returnvalue_2))
                (`UserWidget.AddToViewport` _output_get 0)
                (`KismetSystemLibrary.Delay` 1.0)
                (`UserWidget.PlayAnimation` _infroscreenref (`/Game/Widget/InfoScreen.start` _infroscreenref) 0.0 1 "Forward" 0.5 false)
                (`KismetSystemLibrary.Delay` 9.0)
                (`Widget.SetVisibility` (`self.infroScreenRef`) "Collapsed")
                (`PlayerCameraManager.StartCameraFade` :`self` (`PlayerController.PlayerCameraManager` (`GameplayStatics.GetPlayerController` 0)) :`FromAlpha` 1.0 :`Duration` 1.0))
              (bind _returnvalue_3 (`PrimitiveComponent.CreateDynamicMaterialInstance` (`self.backround`) 0 null "None"))
              (`MaterialInstanceDynamic.SetTextureParameterValue` _returnvalue_3 "tex_1" "/Game/Textures/811038.811038")
              (bind _returnvalue_4 (`|CreateWidget` "/Game/Widget/TitleScreenWidget.TitleScreenWidget_C"))
              (`UserWidget.AddToViewport` _returnvalue_4 0)
              (bind _returnvalue_5 (`GameUserSettings.GetGameUserSettings`))
              (`GameUserSettings.SetVSyncEnabled` _returnvalue_5 true)
              (`GameUserSettings.ApplySettings` _returnvalue_5 false)
              (set `/Game/flat_dark_themed_gui/widgets/sample_windows/ThemeBlack/settings_store/W_SettingsBlack_Sample.LevelBlockManagerRef` self (`/Game/Widget/TitleScreenWidget.W_SettingsBlack_Sample` _returnvalue_4))
              (bind _returnvalue_6 (`GameplayStatics.LoadGameFromSlot` "osou_settings"))
              (bind _assaved_settings_bp_2 (cast `/Game/Blueprints/SavedSettings_BP` _returnvalue_6))
              (`AudioComponent.SetVolumeMultiplier` (`self.a1`) (`/Game/Blueprints/SavedSettings_BP.Master Volume` _assaved_settings_bp_2)))))))
    (:`then_1`
      (switch `int` (`KismetMathLibrary.RandomInteger` 4)
        (:`0`
          (`AudioComponent.SetSound` _a1 "/Game/Music/TitleMusic.TitleMusic"))
        (:`1`
          (`AudioComponent.SetSound` _a1 "/Game/Music/TitleMusic1.TitleMusic1"))
        (:`2`
          (`AudioComponent.SetSound` _a1_2 "/Game/Music/TitleMusic2.TitleMusic2"))
        (:`3`
          (`AudioComponent.SetSound` _a1_2 "/Game/Music/TitleMusic3.TitleMusic3"))))))

(fn `UserConstructionScript`)